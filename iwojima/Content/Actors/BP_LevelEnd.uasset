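; BP_LevelEnd is a level exit trigger with a floating text label.
; Overlapping its Box opens the level named by LevelName if ObjectiveAchieved is set; otherwise the text changes to FailString.
; The construction script sets the label to DisplayLocation, and Tick billboards it by combining a 180-degree offset with the player's control rotation.
; The overlap does not filter which actor triggered it.
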(event `self.Box.OnComponentBeginOverlap`
  (params (OverlappedComponent :type "PrimitiveComponent Object Reference") (OtherActor :type "Actor Object Reference") (OtherComp :type "PrimitiveComponent Object Reference") (OtherBodyIndex :type Integer) (bFromSweep :type Boolean) (SweepResult :type "HitResult Structure (by ref)"))
  (if (`self.objectiveAchieved`)
    (`GameplayStatics.OpenLevel` (`self.levelName`))
    (else
      (`TextRenderComponent.K2_SetText` (`self.TextRender`) (`self.failString`)))))

(event `self.ReceiveTick`
  (params (DeltaSeconds :type "Float (single-precision)"))
  (`SceneComponent.K2_SetWorldRotation` (`self.TextRender`) (`KismetMathLibrary.ComposeRotators` (struct :`Yaw` 180.0) (`Controller.GetControlRotation` (`GameplayStatics.GetPlayerController` 0))) false false))

(fn `UserConstructionScript`
  (`TextRenderComponent.K2_SetText` (`self.TextRender`) (`self.DisplayLocation`)))