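; BP_RonaldDiaC is an actor, apparently for a character named Ronald, that opens a dialogue when the player character enters its TalkC trigger.
; Begin overlap checks for BP_ThirdPersonCharacter, creates a DemoDialogueWidget from InDialogue, shows it and enables mouse cursor, click and mouse-over events.
; End overlap removes the widget and disables those mouse settings, without checking which actor left.
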(event `self.TalkC.OnComponentBeginOverlap`
  (params (OverlappedComponent :type "PrimitiveComponent Object Reference") (OtherActor :type "Actor Object Reference") (OtherComp :type "PrimitiveComponent Object Reference") (OtherBodyIndex :type Integer) (bFromSweep :type Boolean) (SweepResult :type "HitResult Structure (by ref)"))
  (bind _returnvalue (`GameplayStatics.GetPlayerController` 0))
  (cast `/Game/ThirdPerson/Blueprints/BP_ThirdPersonCharacter` OtherActor)
  (bind _returnvalue_2 (`|CreateWidget` "/DialoguePlugin/UI/DemoDialogueWidget.DemoDialogueWidget_C" null (`self.In Dialogue`) null))
  (bind _output_get (set `self.dialog` _returnvalue_2))
  (`UserWidget.AddToPlayerScreen` _output_get 0)
  (set `PlayerController.bEnableMouseOverEvents` true _returnvalue)
  (set `PlayerController.bShowMouseCursor` true _returnvalue)
  (set `PlayerController.bEnableClickEvents` true _returnvalue))

(event `self.TalkC.OnComponentEndOverlap`
  (params (OverlappedComponent :type "PrimitiveComponent Object Reference") (OtherActor :type "Actor Object Reference") (OtherComp :type "PrimitiveComponent Object Reference") (OtherBodyIndex :type Integer))
  (bind _returnvalue (`GameplayStatics.GetPlayerController` 0))
  (`Widget.RemoveFromParent` (`self.dialog`))
  (set `PlayerController.bEnableMouseOverEvents` false _returnvalue)
  (set `PlayerController.bShowMouseCursor` false _returnvalue)
  (set `PlayerController.bEnableClickEvents` false _returnvalue))

(fn `UserConstructionScript`)