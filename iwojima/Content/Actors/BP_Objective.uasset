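; BP_Objective is a level objective that marks the level end's objective as achieved when something overlaps its sphere.
; The overlap finds BP_LevelEnd by class, sets its ObjectiveAchieved flag and updates its TextRender with DisplayLocation, with no filter on the overlapping actor.
; The objective's own Lol text shows the flag's value, set in the construction script and refreshed on overlap.
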(event `self.Sphere1.OnComponentBeginOverlap`
  (params (OverlappedComponent :type "PrimitiveComponent Object Reference") (OtherActor :type "Actor Object Reference") (OtherComp :type "PrimitiveComponent Object Reference") (OtherBodyIndex :type Integer) (bFromSweep :type Boolean) (SweepResult :type "HitResult Structure (by ref)"))
  (bind _returnvalue (`GameplayStatics.GetActorOfClass` "/Game/Actors/BP_LevelEnd.BP_LevelEnd_C"))
  (bind _output_get (set `/Game/Actors/BP_LevelEnd.objectiveAchieved` true _returnvalue))
  (`TextRenderComponent.K2_SetText` (`self.lol`) (`KismetTextLibrary.Conv_BoolToText` _output_get))
  (`TextRenderComponent.K2_SetText` (`/Game/Actors/BP_LevelEnd.TextRender` _returnvalue) (`/Game/Actors/BP_LevelEnd.DisplayLocation` _returnvalue)))

(fn `UserConstructionScript`
  (bind _returnvalue (`GameplayStatics.GetActorOfClass` "/Game/Actors/BP_LevelEnd.BP_LevelEnd_C"))
  (`TextRenderComponent.K2_SetText` (`self.lol`) (`KismetTextLibrary.Conv_BoolToText` (`/Game/Actors/BP_LevelEnd.objectiveAchieved` _returnvalue))))