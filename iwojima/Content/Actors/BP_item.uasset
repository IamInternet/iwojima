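; BP_item is a pickup item actor whose mesh is set from a MeshName variable in the construction script.
; A box overlap flags it as in range and registers it as ItemInRange on an overlapping ALS_AnimMan_Pickup; end overlap clears only its own flag.
; PickUp hides the mesh and disables collision, while Drop moves the actor to a given position and restores both.
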(event `self.Box.OnComponentBeginOverlap`
  (params (OverlappedComponent :type "PrimitiveComponent Object Reference") (OtherActor :type "Actor Object Reference") (OtherComp :type "PrimitiveComponent Object Reference") (OtherBodyIndex :type Integer) (bFromSweep :type Boolean) (SweepResult :type "HitResult Structure (by ref)"))
  (set `self.inRange` true)
  (bind _asals_anim_man_pickup (cast `/Game/AdvancedLocomotionV4/Blueprints/CharacterLogic/ALS_AnimMan_Pickup` OtherActor))
  (set `/Game/AdvancedLocomotionV4/Blueprints/CharacterLogic/ALS_AnimMan_Pickup.itemInRange` self _asals_anim_man_pickup))

(event `PickUp`
  (`SceneComponent.SetVisibility` (`self.StaticMesh`) false true)
  (`self.SetActorEnableCollision` false))

(event `self.Box.OnComponentEndOverlap`
  (params (OverlappedComponent :type "PrimitiveComponent Object Reference") (OtherActor :type "Actor Object Reference") (OtherComp :type "PrimitiveComponent Object Reference") (OtherBodyIndex :type Integer))
  (set `self.inRange` false))

(event `Drop`
  (params (Position :type "Vector Structure"))
  (`self.K2_SetActorLocation` Position)
  (`SceneComponent.SetVisibility` (`self.StaticMesh`) true true)
  (`self.SetActorEnableCollision` true))

(fn `UserConstructionScript`
  (`StaticMeshComponent.SetStaticMesh` (`self.StaticMesh`) (`self.meshName`)))