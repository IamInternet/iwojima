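; BP_CheckpointSystem is an actor that returns the player character to a spawn point after it falls below a death height.
; The construction script stores the actor's own location as the spawn point.
; Each tick it looks up the ALS_AnimMan_CharacterBP instance by class and teleports it there, without sweep, when its Z drops under DeathHeight.
; The spawn point is never updated during play.
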(event `self.ReceiveTick`
  (params (DeltaSeconds :type "Float (single-precision)"))
  (bind _returnvalue (`GameplayStatics.GetActorOfClass` "/Game/AdvancedLocomotionV4/Blueprints/CharacterLogic/ALS_AnimMan_CharacterBP.ALS_AnimMan_CharacterBP_C"))
  (if (< (.z (`self.K2_GetActorLocation` _returnvalue)) (`self.DeathHeight`))
    (`self.K2_SetActorLocation` _returnvalue (`self.Spawn`) false true)))

(fn `UserConstructionScript`
  (set `self.Spawn` (`self.K2_GetActorLocation`)))